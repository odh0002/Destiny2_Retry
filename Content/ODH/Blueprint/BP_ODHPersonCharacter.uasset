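; BP_ODHPersonCharacter is a first-person character Blueprint that adds sprinting and held-trigger rifle firing through Enhanced Input.
; Sprint raises the character's max walk speed while held and lowers it on release.
; Shoot starts a looping timer that replays the rifle montage on the first-person mesh until release clears it.
; Firing is animation only, with no projectile, trace or damage, and an aiming-based montage choice sits unused.
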(event `EnhancedInput|/Game/LJY/Input/Actions/IA_Sprint`
  (params (ActionValue :type Boolean) (ElapsedSeconds :type "Float (double-precision)") (TriggeredSeconds :type "Float (double-precision)") (InputAction :type "InputAction Object Reference" :default "/Game/LJY/Input/Actions/IA_Sprint.IA_Sprint"))
  (bind _charactermovement (`self.CharacterMovement`))
  ; Simple Sprint
  (:`Started`
    (set `CharacterMovementComponent.MaxWalkSpeed` 800.0 _charactermovement))
  (:`Completed`
    (set `CharacterMovementComponent.MaxWalkSpeed` 500.0 _charactermovement)))

(event `EnhancedInput|/Game/LJY/Input/Actions/IA_Shoot`
  (params (ActionValue :type Boolean) (ElapsedSeconds :type "Float (double-precision)") (TriggeredSeconds :type "Float (double-precision)") (InputAction :type "InputAction Object Reference" :default "/Game/LJY/Input/Actions/IA_Shoot.IA_Shoot"))
  (:`Started`
    (bind _returnvalue (`KismetSystemLibrary.K2_SetTimerDelegate` (delegate `FireWeaponEvent`) 0.1 true))
    (set `self.FireTimeRef` _returnvalue))
  (:`Completed`
    (`KismetSystemLibrary.K2_ClearAndInvalidateTimerHandle` (`self.FireTimeRef`))))

(event `FireWeaponEvent`
  (`|PlayMontage` (`self.Mesh1P`) "/Game/FirstPersonArms/Animations/FP_Rifle_Shoot_Montage.FP_Rifle_Shoot_Montage"))

(fn `UserConstructionScript`)