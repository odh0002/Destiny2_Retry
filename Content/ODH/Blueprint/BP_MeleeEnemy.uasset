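; BP_MeleeEnemy is a melee enemy Blueprint whose graph manages a temporary HP bar widget shown when projectiles hit it.
; BeginPlay links the widget to its owning enemy and hides it.
; Overlapping a first-person projectile shows the bar or restarts its timer, hiding it instead if Health is depleted.
; Tick hides the bar once LifeTime elapses; damage is not applied in this graph.
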(event `self.ReceiveBeginPlay`
  ; UI가 주인을 알수 있도록 처음에 지정
  (bind _aswbp_enemy_hpbar (cast `/Game/ODH/Blueprint/WBP_EnemyHPBar` (`WidgetComponent.GetUserWidgetObject` (`self.HPBar`))))
  (set `/Game/ODH/Blueprint/WBP_EnemyHPBar.OwnActor` self _aswbp_enemy_hpbar)
  (`Widget.SetVisibility` _aswbp_enemy_hpbar "Hidden"))

(event `self.ReceiveTick`
  (params (DeltaSeconds :type "Float (single-precision)"))
  (if (`Widget.IsVisible` (stale `self.ReceiveBeginPlay` _aswbp_enemy_hpbar))
    (bind _output_get (set `self.CurTime` (+ (`self.CurTime`) DeltaSeconds)))
    (if (>= _output_get (`self.LifeTime`))
      (`Widget.SetVisibility` (stale `self.ReceiveBeginPlay` _aswbp_enemy_hpbar) "Hidden")
      (set `self.CurTime` 0.0))))

(event `self.ReceiveActorBeginOverlap`
  (params (OtherActor :type "Actor Object Reference"))
  (cast `/Game/FirstPerson/Blueprints/BP_FirstPersonProjectile` OtherActor)
  (if (`Widget.IsVisible` (stale `self.ReceiveBeginPlay` _aswbp_enemy_hpbar))
    ; 체력이 0이 되면 UI 감추기
    (if (<= (`self.Health`) 0.0)
      (`Widget.SetVisibility` (stale `self.ReceiveBeginPlay` _aswbp_enemy_hpbar) "Hidden")
      (else
        (set `self.CurTime` 0.0)))
    (elif (> (`self.Health`) 0.0)
      (`Widget.SetVisibility` (stale `self.ReceiveBeginPlay` _aswbp_enemy_hpbar) "Visible"))))

(fn `UserConstructionScript`)